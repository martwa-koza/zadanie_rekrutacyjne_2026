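; BP_DestructableActor is an interactable prop that the player breaks with a hammer to release loot.
; Overlapping the icon radius while holding the hammer sets HasHammer and swaps the default icon for a hammer icon.
; With that flag set, each interaction plays a timeline yaw shake on the mesh and applies fixed self-damage.
; The health component's death event spawns LootArray classes at the mesh location, calling DestroyActor inside the loop.
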(event OnComponentBeginOverlap(IconRadius)
  (params (OverlappedComponent :type Primitive%20Component%20Object%20Reference) (OtherActor :type Actor%20Object%20Reference) (OtherComp :type Primitive%20Component%20Object%20Reference) (OtherBodyIndex :type Integer) (bFromSweep :type Boolean) (SweepResult :type Hit%20Result%20Structure%20%28by%20ref%29))
  ;[0.15 0.15 0.15 0.5] hammer icon visibility when player has hammer
  (if (Variables|/Game/ThirdPerson/Blueprints/BP_MyCharacter.BP_MyCharacter_C|GetHolds%20Hammer (CallFunction|GetMyCharacter))
    (Variables|Default|SetHas%20Hammer? true)
    (Rendering|SetVisibility (Variables|Default|GetDefault%20Icon) false false)
    (Rendering|SetVisibility (Variables|Default|GetHammer%20Icon) true false)))

(event OnDeath(BP_HealthComponent)
  ;[0.15 0.15 0.15 0.5] Spawn loot on death
  (for _array_element (Variables|Default|GetLoot%20Array)
    (Game|SpawnActorfromClass _array_element (Math|Transform|MakeTransform (Transformation|GetWorldLocation (Variables|Default|GetStaticMesh)) "0, 0, 0" "1.000000,1.000000,1.000000") "Undefined" "MultiplyWithRoot" 0 0)
    (Actor|DestroyActor)))

(event Custom|Shake%20On%20Hit
  ;[0.15 0.15 0.15 0.5] Shake on hit
  (bind _newtrack_0 (Timeline|Shake%20Timeline PlayFromStart)
    (:Update
      (Transformation|SetRelativeRotation (Variables|Default|GetStaticMesh) (Math|Rotator|MakeRotator 0.0 0.0 _newtrack_0) false false))))

(event EventInteraction
  ;[0.15 0.15 0.15 0.5] Event interact
  (if (Variables|Default|GetHas%20Hammer?)
    (CallFunction|ShakeonHit)
    (Game|Damage|ApplyDamage self 25.0 0 0)))

(fn ConstructionScript
  (|CallParentFunction)
  ;[0.15 0.15 0.15 0.5] hammer icon details
  (Transformation|SetWorldScale3D (Variables|Default|GetHammer%20Icon) (Math|Conversions|ToVector(Float) (Variables|Default|GetHammer%20Icon%20Scale)))
  (Rendering|SetVisibility (Variables|Default|GetHammer%20Icon) false false))