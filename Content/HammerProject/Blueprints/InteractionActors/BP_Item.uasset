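; BP_Item is an interactable world item that destroys itself when used and shows an icon when the player is nearby.
; The IconRadius overlap events unhide DefaultIcon when the player character enters and hide it again on exit.
; The Interaction event prints a debug string, then destroys the actor after a short delay.
; The construction script applies the IconScale variable to the icon's world scale.
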(event OnComponentBeginOverlap(IconRadius)
  (params (OverlappedComponent :type Primitive%20Component%20Object%20Reference) (OtherActor :type Actor%20Object%20Reference) (OtherComp :type Primitive%20Component%20Object%20Reference) (OtherBodyIndex :type Integer) (bFromSweep :type Boolean) (SweepResult :type Hit%20Result%20Structure%20%28by%20ref%29))
  ;[0.15 0.15 0.15 0.5] Icon radius - show icon on overlap
  (if (== OtherActor (Game|GetPlayerCharacter 0))
    (Development|SetHiddeninGame (Variables|Default|GetDefault%20Icon) false false)))

(event OnComponentEndOverlap(IconRadius)
  (params (OverlappedComponent :type Primitive%20Component%20Object%20Reference) (OtherActor :type Actor%20Object%20Reference) (OtherComp :type Primitive%20Component%20Object%20Reference) (OtherBodyIndex :type Integer))
  ;[0.15 0.15 0.15 0.5] Icon radius - hide icon on end overlap
  (if (== OtherActor (Game|GetPlayerCharacter 0))
    (Development|SetHiddeninGame (Variables|Default|GetDefault%20Icon) true false)))

(event EventInteraction
  ;[0.15 0.15 0.15 0.5] Destroy actor on interaction
  (Development|PrintString "Interacted")
  (Utilities|FlowControl|Delay 0.2)
  (Actor|DestroyActor))

(fn ConstructionScript
  ;[0.15 0.15 0.15 0.5] Set icon scale
  (Transformation|SetWorldScale3D (Variables|Default|GetDefault%20Icon) (Math|Conversions|ToVector(Float) (Variables|Default|GetIcon%20Scale))))